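; Spline cart actor that travels along the track of a referenced spline actor when active at BeginPlay.
; A timeline, with play rate scaled by the inverse of a duration and started at a configurable offset, drives an alpha over the spline length.
; Each update moves and rotates the cart to the world-space location and rotation at that distance.
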(event `self.ReceiveBeginPlay`
  ;[1 1 1] Will move the cart along the spline as long as it is active
  (if (`self.ActiveCart`)
    (`self.MoveCart`)))

(event `MoveCart`
  (bind _returnvalue (`KismetMathLibrary.Lerp` 0.0 (`SplineComponent.GetSplineLength` (`/Game/UNISession/Blueprints/SplineTrack.SplineTrack` (`self.SplineRef`))) (`self.Alpha`)))
  ;[1 1 1] Creates a timeline for the cart, allowing it to move across the spline at the given duration
  (`TimelineComponent.SetPlayRate` (`self.Movement`) (/ 1.0 (`self.Duration`)))
  (`TimelineComponent.SetNewTime` (`self.Movement`) (`self.CartStartOffset`))
  (bind (_direction _alpha) (`Timeline|Movement`)
    (:`Update`
      (set `self.Alpha` _alpha)
      (`self.K2_SetActorLocationAndRotation` (`SplineComponent.GetLocationAtDistanceAlongSpline` (`/Game/UNISession/Blueprints/SplineTrack.SplineTrack` (`self.SplineRef`)) _returnvalue "World") (`SplineComponent.GetRotationAtDistanceAlongSpline` (`/Game/UNISession/Blueprints/SplineTrack.SplineTrack` (`self.SplineRef`)) _returnvalue "World")))))

(fn `UserConstructionScript`)