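; An AI pawn that roams at random and chases the ThirdPersonCharacter when it sees it.
; PawnSensing's see event sets the chase flags and moves toward the player, with a retriggerable delay clearing them shortly after sightings stop.
; While not chasing, Tick uses random delays before AIMoveTo sends it to a reachable point within a radius of its location.
; Only sight is wired, despite a comment mentioning hearing.
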(event `self.ReceiveTick`
  (params (DeltaSeconds :type "Float (single-precision)"))
  (`|ExecutionSequence`
    (:`then_0`
      ;[1 1 1] Set to see if AI has lost line of sight of player
      (if (not (`self.CanSeeEnemy?`))
        (`KismetSystemLibrary.Delay` 0.4)
        (set `self.IsChasing?` false)))
    (:`then_1`
      (if (not (`self.IsChasing?`))
        ;[1 1 1] AI Random Roaming
        (`KismetSystemLibrary.Delay` (`KismetMathLibrary.RandomFloatInRange` 1.0 5.0))
        (set `self.IsMoving?` true)
        (`|AIMoveTo` self (`NavigationSystemV1.K2_GetRandomReachablePointInRadius` (`self.K2_GetActorLocation`) 1500.0 null null) null
          (:`OnSuccess`
            _)
          (:`OnFail`
            _))
        (set `self.IsMoving?` false)))))

(event `self.PawnSensing.OnSeePawn`
  (params (Pawn :type "Pawn Object Reference"))
  ;[1 1 1] Using pawn sensing to allow the AI to see and hear the player
  (bind _asthird_person_character (cast `/Game/UNISession/Blueprints/ThirdPersonCharacter` Pawn))
  (`|ExecutionSequence`
    (:`then_0`
      (set `self.CanSeeEnemy?` true)
      (set `self.IsChasing?` true)
      (`|AIMoveTo` self (0.0 0.0 0.0) _asthird_person_character))
    (:`then_1`
      (`KismetSystemLibrary.RetriggerableDelay` 0.6)
      (set `self.CanSeeEnemy?` false)
      (set `self.IsChasing?` false))))

(fn `UserConstructionScript`)