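; AI flying shooter actor that turns to face a sensed ThirdPersonCharacter and fires at it.
; PawnSensing drives the look-at rotation and spawns FirstPersonProjectiles, launched by impulse along the Cube's forward vector, with a delay-based cooldown.
; BeginPlay caches three patrol positions and picks a random one.
; The timeline that lerps between random patrol points is never started, so the patrol does not run.
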(event `self.PawnSensing.OnSeePawn`
  (params (Pawn :type "Pawn Object Reference"))
  ;[1 1 1] Look at player and shoot at them
  (bind _asthird_person_character (cast `/Game/UNISession/Blueprints/ThirdPersonCharacter` Pawn))
  (`|ExecutionSequence`
    (:`then_0`
      (`self.K2_SetActorRotation` (`KismetMathLibrary.FindLookAtRotation` (`self.K2_GetActorLocation`) (`self.K2_GetActorLocation` _asthird_person_character))))
    (:`then_1`
      (if (`self.CanShoot`)
        (bind _returnvalue (`|SpawnActorFromClass` "/Game/Projectile/Blueprints/FirstPersonProjectile.FirstPersonProjectile_C" (`SceneComponent.K2_GetComponentToWorld` (`self.ProjectileSpawn`)) "Undefined" "OverrideRootScale" null null))
        (`PrimitiveComponent.AddImpulse` (`/Game/Projectile/Blueprints/FirstPersonProjectile.Sphere` _returnvalue) (* (`SceneComponent.GetForwardVector` (`self.Cube`)) (`self.ShootForce`)) "None" true)
        (set `self.CanShoot` false)
        (`KismetSystemLibrary.Delay` 1.5)
        (set `self.CanShoot` true)))))

(event `self.ReceiveBeginPlay`
  ;[1 1 1] Set patrol points
  (set `self.Patrolpoints` (`|MakeArray` (`SceneComponent.K2_GetComponentLocation` (`self.MovePosition1`)) (`SceneComponent.K2_GetComponentLocation` (`self.MovePosition2`)) (`SceneComponent.K2_GetComponentLocation` (`self.MovePosition3`))))
  (`self.GetRandomLocation`))

(fn `GetRandomLocation`
  (set `self.CurrentPatrolPoint` (`KismetMathLibrary.RandomInteger` (`KismetArrayLibrary.Array_Length` (`self.Patrolpoints`)))))

(fn `UserConstructionScript`)