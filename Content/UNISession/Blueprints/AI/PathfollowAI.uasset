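; AI controller that walks a SpecificPath_AI pawn along a linked chain of path nodes.
; BeginPlay caches the possessed pawn, avoiding a cast on Tick, and starts a move without pathfinding to its DesiredNode.
; Tick polls move status; whenever it differs from DesiredStatus, it advances DesiredNode to its NextNode, then issues a default MoveToActor to the node after that.
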(event `self.ReceiveBeginPlay`
  ;[1 1 1] Starts by getting a reference to the pawn and then starting the movement. This is much better than casting into a tick as it has a much lower resource cost
  (bind _asspecific_path_ai (cast `/Game/UNISession/Blueprints/AI/SpecificPath_AI` (`self.K2_GetPawn`)))
  (bind _output_get (set `self.StoredPawn` _asspecific_path_ai))
  (`self.MoveToActor` (`/Game/UNISession/Blueprints/AI/SpecificPath_AI.DesiredNode` _output_get) 15.0 true false true null))

(event `self.ReceiveTick`
  (params (DeltaSeconds :type "Float (single-precision)"))
  (bind _storedpawn (`self.StoredPawn`))
  (bind _nextnode (`/Game/UNISession/Blueprints/AI_Helpers/PathNode.NextNode` (`/Game/UNISession/Blueprints/AI/SpecificPath_AI.DesiredNode` _storedpawn)))
  ;[1 1 1] Blueprint implementation for AI PathFollowing
  (if (!= (`self.GetMoveStatus`) (`self.DesiredStatus`))
    (set `/Game/UNISession/Blueprints/AI/SpecificPath_AI.DesiredNode` _nextnode _storedpawn)
    (`self.MoveToActor` _nextnode 15.0 true true true null)))

(fn `UserConstructionScript`)